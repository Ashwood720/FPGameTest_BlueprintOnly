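; AI controller for NPCs that runs the BT_NPC behavior tree on possess and feeds it perception results.
; When AI Perception updates, any actor whose class is exactly BP_FirstPersonCharacter is written to the "Enemy" blackboard key.
; The live logic ignores whether sensing succeeded and never clears that key; a sight-specific branch that checks this is left disconnected.
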(event `self.AIPerception.OnTargetPerceptionUpdated`
  (params (Actor :type "Actor Object Reference") (Stimulus :type "AIStimulus Structure")))

(event `self.ReceivePossess`
  (params (PossessedPawn :type "Pawn Object Reference"))
  (`self.RunBehaviorTree` "/Game/AI/ThirdPerson/Blueprints/BT_NPC.BT_NPC"))

(event `self.AIPerception.OnPerceptionUpdated`
  (params (UpdatedActors :type "Array of Actor Object Reference (by ref)"))
  (for _array_element UpdatedActors
    (if (== (`GameplayStatics.GetObjectClass` _array_element) "/Game/FirstPerson/Blueprints/BP_FirstPersonCharacter.BP_FirstPersonCharacter_C")
      (`BlackboardComponent.SetValueAsObject` (`AIBlueprintHelperLibrary.GetBlackboard` null) (`KismetStringLibrary.Conv_StringToName` "Enemy") _array_element))))

(fn `UserConstructionScript`)